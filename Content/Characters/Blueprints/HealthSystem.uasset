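; HealthSystem is a Blueprint that tracks health and mirrors it on a health bar.
; Damage and Heal adjust Health, clamp it to a fixed range and push the normalized value to the Healthbar percent.
; Damage also calls OnDeath whenever health is at zero and returns whether that is the case.
; All logic lives in these two functions, with no active BeginPlay or Tick.
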(event EventBeginPlay)

(event EventTick
  (params (DeltaSeconds :type Float%20%28single-precision%29)))

(fn Damage
  (params (amount :type Float%20%28double-precision%29))
  (bind _output_get (Variables|Default|Sethealth (Math|Float|Clamp(Float) (- (Variables|Default|Gethealth) amount) 0.0 1e+02)))
  (Progress|SetPercent (Variables|Default|Gethealthbar) (/ _output_get 1e+02))
  (if (<= _output_get 0.0)
    (Default|CallOnDeath))
  (return (<= _output_get 0.0)))

(fn Heal
  (params (amount :type Float%20%28double-precision%29))
  (bind _output_get (Variables|Default|Sethealth (Math|Float|Clamp(Float) (+ (Variables|Default|Gethealth) amount) 0.0 1e+02)))
  (Progress|SetPercent (Variables|Default|Gethealthbar) (/ _output_get 1e+02))
  (return))