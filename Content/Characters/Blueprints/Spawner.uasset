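; Spawner actor that periodically spawns actors of a configurable class inside a region volume.
; StartSpawning runs a looping timer at the spawn interval, and StopSpawning clears it.
; Each tick picks a random point within the SpawnRegion bounds, spawns there with the owner as instigator, adjusting or skipping on collision, then calls the Spawned dispatcher with the result.
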(event Custom|StopSpawning
  (Utilities|Time|ClearandInvalidateTimerbyHandle (stale Custom|StartSpawning _returnvalue)))

(event Custom|OnSpawn
  (CallFunction|Spawn (stale Custom|StartSpawning owner)))

(event Custom|StartSpawning
  (params (owner :type Pawn%20Object%20Reference))
  (bind _returnvalue (Utilities|Time|SetTimerbyEvent (delegate Custom|OnSpawn) (Variables|Default|Getspawn%20interval) true)))

(fn ConstructionScript)

(fn Spawn
  (params (owner :type Pawn%20Object%20Reference))
  (bind _spawn_region (Variables|Default|Getspawn%20region))
  (bind (_origin _boxextent) (Collision|GetComponentBounds _spawn_region))
  (bind _returnvalue (Game|SpawnActorfromClass (Variables|Default|Getspawned%20actor%20class) (Math|Conversions|ToTransform(Vector) (Math|Random|RandomPointinBoundingBox _origin _boxextent)) "AdjustIfPossibleButDontSpawnIfColliding" "MultiplyWithRoot" 0 owner))
  (Default|CallSpawned _returnvalue)
  (return _returnvalue))