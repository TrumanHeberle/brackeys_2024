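; Base character Blueprint that displays a name label and responds to interaction events.
; The construction script fills the text component from CharacterName.
; SetInteractableState shows or hides that label based on whether interaction can be shown.
; StopInteraction forwards the call to the stored InteractInstigator, and the default BeginPlay, overlap and Tick events are unused.
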(event EventBeginPlay)

(event Collision|EventActorBeginOverlap
  (params (OtherActor :type Actor%20Object%20Reference)))

(event EventTick
  (params (DeltaSeconds :type Float%20%28single-precision%29)))

(event EventStopInteraction
  (Default|StopInteraction (Variables|Default|GetInteractInstigator)))

(event EventSetInteractableState
  (params (CanShowInteract? :type Boolean))
  (if CanShowInteract?
    (Rendering|SetVisibility (Variables|Default|GetTxt_CharacterName) true false)
    (else
      (Rendering|SetVisibility (Variables|Default|GetTxt_CharacterName) false false))))

(fn ConstructionScript
  (Rendering|Components|TextRender|SetText (Variables|Default|GetTxt_CharacterName) (Variables|Default|GetCharacterName)))